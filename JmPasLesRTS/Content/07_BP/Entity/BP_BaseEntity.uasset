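; BP_BaseEntity is a base entity with a faction, a move-to-point action and an attack cooldown, driven through AIC_BaseAIController.
; On BeginPlay it applies the Ally or Enemy material to its mesh, printing a warning for Neutral.
; PrimaryAction passes the hit location to the controller as a target, and ResetAttack disables the controller's attacking until AttackDelay elapses.
; Attack and IsSelect are placeholders that only print or return false.
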(event `self.ReceiveBeginPlay`
  (`self.SetTeamColor`))

(event `/Game/07_BP/BPI_Select.PrimaryAction`
  (params (Hit :type "HitResult Structure"))
  (bind _asaic_base_aicontroller (cast `/Game/07_BP/Entity/AI/AIC_BaseAIController` (`self.GetController`)))
  (`/Game/07_BP/Entity/AI/AIC_BaseAIController.SetTargetLocation` _asaic_base_aicontroller (`.Location` (`GameplayStatics.BreakHitResult` Hit))))

(event `ResetAttack`
  (bind _asaic_base_aicontroller (cast `/Game/07_BP/Entity/AI/AIC_BaseAIController` (`self.GetController`)))
  (`/Game/07_BP/Entity/AI/AIC_BaseAIController.SetCanAttack` _asaic_base_aicontroller false)
  (`KismetSystemLibrary.Delay` (`self.AttackDelay`))
  (`/Game/07_BP/Entity/AI/AIC_BaseAIController.SetCanAttack` _asaic_base_aicontroller true))

(fn `Attack`
  (`KismetSystemLibrary.PrintString` "Attack"))

(fn `IsSelect`
  (returns (IsSelect :type Boolean))
  (return false))

(fn `SetTeamColor`
  (bind _staticmesh (`self.StaticMesh`))
  (switch `/Game/07_BP/Entity/E_Faction` (`self.Faction`)
    (:`NewEnumerator0`
      (`KismetSystemLibrary.PrintString` "TeamNotAssign" true true (struct :`R` 1.0 :`G` 0.074453 :`A` 1.0)))
    (:`NewEnumerator1`
      (`PrimitiveComponent.SetMaterial` _staticmesh 0 (`self.MatAlly`)))
    (:`NewEnumerator2`
      (`PrimitiveComponent.SetMaterial` _staticmesh 0 (`self.MatEnemy`)))))

(fn `UserConstructionScript`)