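; BP_HuvaController is a player controller that tracks which actor is under the mouse cursor and sends it hover notifications.
; Every Tick it stores a complex Visibility trace under the cursor, then runs HoverUpdate to compare the hit actor with the cached HoverActor.
; When the target changes, it sends unhover to the old actor and hover to the new one, for actors implementing BPI_Select.
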(event `self.ReceiveTick`
  (params (DeltaSeconds :type "Float (single-precision)"))
  (set `self.HitCursor` (`self.GetHitResultUnderCursorByChannel` "TraceTypeQuery1"))
  (`self.HoverUpdate`))

(fn `HoverUpdate`
  (bind _hoveractor (`self.HoverActor`))
  (bind (_bblockinghit _binitialoverlap _time _distance _location _impactpoint _normal _impactnormal _physmat _hitactor) (`GameplayStatics.BreakHitResult` (`self.HitCursor`)))
  (`/Engine/EditorBlueprintResources/StandardMacros.IsValid` _hoveractor
    (:`Is Valid`
      (if (!= _hoveractor _hitactor)
        (if (`KismetSystemLibrary.DoesImplementInterface` (`self.HoverActor`) "/Game/07_BP/BPI_Select.BPI_Select_C")
          (message `/Game/07_BP/BPI_Select.OnUnHover` (`self.HoverActor`)))
        (set `self.HoverActor` _hitactor :!label _label)
        (if (`KismetSystemLibrary.DoesImplementInterface` (`self.HoverActor`) "/Game/07_BP/BPI_Select.BPI_Select_C")
          (message `/Game/07_BP/BPI_Select.OnHover` (`self.HoverActor`)))))
    (:`Is Not Valid`
      (goto _label))))

(fn `UserConstructionScript`)