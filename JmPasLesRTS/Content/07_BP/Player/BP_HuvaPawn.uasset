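; BP_HuvaPawn is a player pawn that handles mouse hover and click selection of actors in the world.
; Each Tick it traces under the cursor through BP_HuvaController, and HoverUpdate sends BPI_Select hover and unhover messages when the hit actor changes.
; A left click on a selectable hovered actor moves the single selection to it, or toggles selection if it is already the selected one.
; CallOnNewSelect calls exist but are unconnected.
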(event `self.ReceiveBeginPlay`
  (bind _asbp_huva_controller (cast `/Game/07_BP/Player/BP_HuvaController` (`self.GetController`)))
  (set `self.ControllerRef` _asbp_huva_controller))

(event `self.ReceiveTick`
  (params (DeltaSeconds :type "Float (single-precision)"))
  (set `self.HitCursor` (`PlayerController.GetHitResultUnderCursorByChannel` (`self.ControllerRef`) "TraceTypeQuery1" true))
  (`self.HoverUpdate`))

(event `InputAction|LeftMouse`
  (params (Key :type "Key Structure"))
  (bind _hoveractor (`self.HoverActor`))
  (bind _hoveractor_2 (`self.HoverActor`))
  (:`Pressed`
    (if (`KismetSystemLibrary.DoesImplementInterface` _hoveractor "/Game/07_BP/BPI_Select.BPI_Select_C")
      (`/Engine/EditorBlueprintResources/StandardMacros.IsValid` (`self.SelectActor`)
        (:`Is Valid`
          (if (!= _hoveractor (`self.SelectActor`))
            (message `/Game/07_BP/BPI_Select.OnUnSelect` (`self.SelectActor`))
            (bind _output_get (set `self.SelectActor` (`self.HoverActor`)))
            (message `/Game/07_BP/BPI_Select.OnSelect` _output_get)
            (else
              (bind _isselect (message `/Game/07_BP/BPI_Select.IsSelect` _hoveractor_2))
              (if _isselect
                (message `/Game/07_BP/BPI_Select.OnUnSelect` _hoveractor_2)
                (else
                  (message `/Game/07_BP/BPI_Select.OnSelect` _hoveractor_2 :!label _label)
                  (set `self.SelectActor` (`self.HoverActor`)))))))
        (:`Is Not Valid`
          (goto _label))))))

(fn `HoverUpdate`
  (bind _hoveractor (`self.HoverActor`))
  (bind (_bblockinghit _binitialoverlap _time _distance _location _impactpoint _normal _impactnormal _physmat _hitactor) (`GameplayStatics.BreakHitResult` (`self.HitCursor`)))
  (`/Engine/EditorBlueprintResources/StandardMacros.IsValid` _hoveractor
    (:`Is Valid`
      (if (!= _hoveractor _hitactor)
        (if (`KismetSystemLibrary.DoesImplementInterface` (`self.HoverActor`) "/Game/07_BP/BPI_Select.BPI_Select_C")
          (message `/Game/07_BP/BPI_Select.OnUnHover` (`self.HoverActor`)))
        (set `self.HoverActor` _hitactor :!label _label)
        (if (`KismetSystemLibrary.DoesImplementInterface` (`self.HoverActor`) "/Game/07_BP/BPI_Select.BPI_Select_C")
          (message `/Game/07_BP/BPI_Select.OnHover` (`self.HoverActor`)))))
    (:`Is Not Valid`
      (goto _label))))

(fn `UserConstructionScript`)