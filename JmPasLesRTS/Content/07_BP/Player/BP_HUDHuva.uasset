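; HUD for the Huva pawn that creates the heads-up display widget and handles drag-box selection of allied entities.
; While the pawn is box-selecting, DrawHUD draws a rectangle from the projected first world hit point to the mouse, keeping it world-anchored.
; Each frame it syncs the pawn's SelectEntities with that rectangle, adding Ally-faction BP_BaseEntity actors and dropping BPI_Select actors outside it.
; Selection outlines toggle custom depth on static mesh components.
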(event `self.ReceiveBeginPlay`
  (bind _asbp_huva_pawn (cast `/Game/07_BP/Player/BP_HuvaPawn` (`GameplayStatics.GetPlayerPawn` 0)))
  (set `self.PawnRef` _asbp_huva_pawn)
  (bind _returnvalue (`|CreateWidget` "/Game/06_Widget/WBP_HeadsUpDisplay.WBP_HeadsUpDisplay_C"))
  (bind _output_get (set `self.HeadsUpDisplay` _returnvalue))
  (`UserWidget.AddToViewport` _output_get 0))

(event `self.ReceiveDrawHUD`
  (params (SizeX :type Integer) (SizeY :type Integer))
  (bind _pawnref (`self.PawnRef`))
  (bind _controllerref (`/Game/07_BP/Player/BP_HuvaPawn.ControllerRef` _pawnref))
  (bind (_locationx _locationy) (`PlayerController.GetMousePosition` _controllerref))
  (bind _screenposition (`GameplayStatics.ProjectWorldToScreen` _controllerref (`/Game/07_BP/Player/BP_HuvaPawn.FirstHitWorldPoint` _pawnref) true))
  (bind (_locationx_2 _locationy_2) (`PlayerController.GetMousePosition` (`/Game/07_BP/Player/BP_HuvaPawn.ControllerRef` (`self.PawnRef`))))
  (bind (_x _y) (`KismetMathLibrary.BreakVector2D` _screenposition))
  (bind _outactors (`self.GetActorsInSelectionRectangle` "/Script/Engine.Actor" _screenposition (`KismetMathLibrary.MakeVector2D` _locationx_2 _locationy_2) false))
  (if (`/Game/07_BP/Player/BP_HuvaPawn.IsSelectInRectangle` _pawnref)
    (if (> (`KismetMathLibrary.Distance2D` (`KismetMathLibrary.MakeVector2D` _locationx _locationy) _screenposition) 5.0)
      (`self.DrawLine` _x _y _locationx _y (struct :`R` 1.0 :`G` 1.0 :`B` 1.0 :`A` 1.0) 1.0)
      (`self.DrawLine` _x _y _x _locationy (struct :`R` 1.0 :`G` 1.0 :`B` 1.0 :`A` 1.0) 1.0)
      (`self.DrawLine` _x _locationy _locationx _locationy (struct :`R` 1.0 :`G` 1.0 :`B` 1.0 :`A` 1.0) 1.0)
      (`self.DrawLine` _locationx _y _locationx _locationy (struct :`R` 1.0 :`G` 1.0 :`B` 1.0 :`A` 1.0) 1.0))
    (for _array_element (`/Game/07_BP/Player/BP_HuvaPawn.SelectEntities` (`self.PawnRef`))
      (if (`KismetSystemLibrary.DoesImplementInterface` _array_element "/Game/07_BP/BPI_Select.BPI_Select_C")
        (if (not (`KismetArrayLibrary.Array_Contains` _outactors _array_element))
          (`self.UpdateActorOutline` _array_element)
          (`KismetArrayLibrary.Array_RemoveItem` (`/Game/07_BP/Player/BP_HuvaPawn.SelectEntities` (`self.PawnRef`)) _array_element))))
    (for _array_element_2 _outactors
      (bind _asbp_base_entity (cast `/Game/07_BP/Entity/BP_BaseEntity` _array_element_2))
      (if (not (`KismetArrayLibrary.Array_Contains` (`/Game/07_BP/Player/BP_HuvaPawn.SelectEntities` (`self.PawnRef`)) _asbp_base_entity))
        (switch `/Game/07_BP/Entity/E_Faction` (`/Game/07_BP/BPAC_HealthFaction.Faction` (`/Game/07_BP/Entity/BP_BaseEntity.BPAC_HealthFaction` _asbp_base_entity))
          (:`NewEnumerator1`
            (`KismetArrayLibrary.Array_Add` (`/Game/07_BP/Player/BP_HuvaPawn.SelectEntities` (`self.PawnRef`)) _asbp_base_entity)
            (`self.UpdateActorOutline` _asbp_base_entity true)))))))

(fn `UpdateActorOutline`
  (params (Actors :type "Actor Object Reference") (IsSelect :type Boolean))
  (for _array_element (`self.K2_GetComponentsByClass` Actors "/Script/Engine.StaticMeshComponent")
    (`PrimitiveComponent.SetRenderCustomDepth` _array_element IsSelect)))

(fn `UpdateActorsOutline`
  (params (Actors :type "Array of Actor Object Reference") (IsSelect :type Boolean))
  (for _array_element Actors
    (`self.UpdateActorOutline` _array_element IsSelect)))

(fn `UserConstructionScript`)